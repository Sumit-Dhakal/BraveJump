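; BP_Lvl2 is a trigger actor that gates the transition to Level2 behind coin collection.
; When an actor tagged Knight overlaps its Box, it compares the player knight_BP's Coins with BP_GameMode's Totalcoins.
; An exact match opens Level2 by name, and any other count creates an InsufficientCoin widget and adds it to the viewport.
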(event `self.Box.OnComponentBeginOverlap`
  (params (OverlappedComponent :type "PrimitiveComponent Object Reference") (OtherActor :type "Actor Object Reference") (OtherComp :type "PrimitiveComponent Object Reference") (OtherBodyIndex :type Integer) (bFromSweep :type Boolean) (SweepResult :type "HitResult Structure (by ref)"))
  (if (`self.ActorHasTag` OtherActor "Knight")
    (bind _asknight_bp (cast `/Game/Blueprints/knight_BP` (`GameplayStatics.GetPlayerCharacter` 0)))
    (bind _asbp_game_mode (cast `/Game/Blueprints/BP_GameMode` (`GameplayStatics.GetGameMode`)))
    (if (== (`/Game/Blueprints/knight_BP.Coins` _asknight_bp) (`/Game/Blueprints/BP_GameMode.totalcoins` _asbp_game_mode))
      (`GameplayStatics.OpenLevel` "Level2")
      (else
        (bind _returnvalue (`|CreateWidget` "/Game/UI/InsufficientCoin.InsufficientCoin_C"))
        (`UserWidget.AddToViewport` _returnvalue 0)))))

(fn `UserConstructionScript`)