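; BP_Enemy is a slime enemy that paces along the X axis until a knight kills it.
; Tick moves it constantly, while capsule hits toggle direction through a FlipFlop, though both branches set identical sprite rotation.
; A "Knight"-tagged overlap on Getdamage triggers, once, a death flipbook, a short delay, destruction, an explosion sound and a LaunchCharacter call along the knight's up vector.
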(event `self.ReceiveTick`
  (params (DeltaSeconds :type "Float (single-precision)"))
  (`self.AddMovementInput` (`self.World Direction`)))

(event `Change Move`
  (`/Engine/EditorBlueprintResources/StandardMacros.FlipFlop`
    (:`A`
      (`SceneComponent.K2_SetWorldRotation` (`self.Sprite`) (struct :`Yaw` -180.0) false false)
      (set `self.World Direction` (-1.0 0.0 0.0)))
    (:`B`
      (`SceneComponent.K2_SetWorldRotation` (`self.Sprite`) (struct :`Yaw` -180.0) false false)
      (set `self.World Direction` (1.0 0.0 0.0)))))

(event `self.CapsuleComponent.OnComponentHit`
  (params (HitComponent :type "PrimitiveComponent Object Reference") (OtherActor :type "Actor Object Reference") (OtherComp :type "PrimitiveComponent Object Reference") (NormalImpulse :type "Vector Structure") (Hit :type "HitResult Structure (by ref)"))
  (`self.Change Move`))

(event `self.getdamage.OnComponentBeginOverlap`
  (params (OverlappedComponent :type "PrimitiveComponent Object Reference") (OtherActor :type "Actor Object Reference") (OtherComp :type "PrimitiveComponent Object Reference") (OtherBodyIndex :type Integer) (bFromSweep :type Boolean) (SweepResult :type "HitResult Structure (by ref)"))
  (if (`self.ActorHasTag` OtherActor "Knight")
    (`/Engine/EditorBlueprintResources/StandardMacros.DoOnce` false
      (:`Completed`
        (`PaperFlipbookComponent.SetFlipbook` (`self.Sprite`) "/Game/Sprites/Enemy/Slime_death.Slime_death")
        (`KismetSystemLibrary.Delay` 0.2)
        (`self.K2_DestroyActor`)
        (`GameplayStatics.PlaySound2D` "/Game/sound/explosion.explosion" 1.0 1.0 0.0 null null)
        (bind _asknight_bp (cast `/Game/Blueprints/knight_BP` OtherActor))
        (`self.LaunchCharacter` (* (`KismetMathLibrary.GetUpVector` (`self.K2_GetActorRotation` _asknight_bp)) 800.0))))))

(fn `UserConstructionScript`)