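; Player-controlled 2D Paper2D knight with side-scrolling movement, jumping, death and pausing.
; BeginPlay adds input mapping and a HUD holding a knight reference; movement and jump also accept externally drivable flags and events.
; Tick selects flipbooks from death, falling and velocity; Damagebox overlap or Fallen triggers one-time death, detaching the camera before GameOver.
; Pause branches on IsPaused to open or close PauseMenu, but never sets it true here.
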(event `self.ReceiveBeginPlay`
  (bind _asplayer_controller (cast `PlayerController` (`self.GetController`)))
  (bind _returnvalue (pcsubsystem `EnhancedInputLocalPlayerSubsystem` _asplayer_controller))
  (`/Engine/EditorBlueprintResources/StandardMacros.IsValid` _returnvalue
    (:`Is Valid`
      (`EnhancedInputSubsystemInterface.AddMappingContext` _returnvalue "/Game/Input/Controls_IMC.Controls_IMC" 0 (struct))
      (bind _returnvalue_2 (`|CreateWidget` "/Game/Blueprints/HUD_WID.HUD_WID_C" null self))
      (bind _output_get (set `self.hud` _returnvalue_2))
      (`UserWidget.AddToViewport` _output_get 0))))

(event `HandleAnim`
  (bind _charactermovement (`self.CharacterMovement`))
  (if (`self.IsDead`)
    (`PaperFlipbookComponent.SetLooping` (`self.Sprite`) false)
    (`PaperFlipbookComponent.SetFlipbook` (`self.Sprite`) "/Game/Sprites/Knight/Knight_death.Knight_death")
    (`/Engine/EditorBlueprintResources/StandardMacros.DoOnce` false
      (:`Completed`
        (`GameplayStatics.PlaySound2D` "/Game/sound/hurt.hurt" 1.0 1.0 0.0 null null)))
    (elif (`NavMovementComponent.IsFalling` _charactermovement)
      (`PaperFlipbookComponent.SetFlipbook` (`self.Sprite`) "/Game/Sprites/Knight/Knight_jump.Knight_jump")
      (elif (> (`KismetMathLibrary.VSize` (`MovementComponent.Velocity` _charactermovement)) 0.0)
        (`PaperFlipbookComponent.SetFlipbook` (`self.Sprite`) "/Game/Sprites/Knight/Knight_Run.Knight_Run")
        (else
          (`PaperFlipbookComponent.SetFlipbook` (`self.Sprite`) "/Game/Sprites/Knight/Kinght_Idle.Kinght_Idle"))))))

(event `self.ReceiveTick`
  (params (DeltaSeconds :type "Float (single-precision)"))
  (`|ExecutionSequence`
    (:`then_0`
      (`self.HandleAnim`))
    (:`then_1`
      (if (`self.Left go?`)
        (`self.AddMovementInput` (-1.0 0.0 0.0))
        (`SceneComponent.K2_SetWorldRotation` (`self.Sprite`) (`KismetMathLibrary.MakeRotator` 0.0 0.0 180.0) false false)))
    (:`then_2`
      (if (`self.right go?`)
        (`self.AddMovementInput` (1.0 0.0 0.0))
        (`SceneComponent.K2_SetWorldRotation` (`self.Sprite`) (`KismetMathLibrary.MakeRotator` 0.0) false false)))))

(event `EnhancedInput|/Game/Input/Move_IA`
  (params (ActionValue :type "Float (double-precision)") (ElapsedSeconds :type "Float (double-precision)") (TriggeredSeconds :type "Float (double-precision)") (InputAction :type "InputAction Object Reference" :default "/Game/Input/Move_IA.Move_IA"))
  (:`Triggered`
    (if (not (`self.IsDead`))
      (`self.AddMovementInput` (1.0 0.0 0.0) ActionValue)
      (`SceneComponent.K2_SetWorldRotation` (`self.Sprite`) (`KismetMathLibrary.MakeRotator` 0.0 0.0 (`KismetMathLibrary.SelectFloat` 0.0 180.0 (> ActionValue 0.3))) false false))))

(event `EnhancedInput|/Game/Input/Jump_IA`
  (params (ActionValue :type Boolean) (ElapsedSeconds :type "Float (double-precision)") (TriggeredSeconds :type "Float (double-precision)") (InputAction :type "InputAction Object Reference" :default "/Game/Input/Jump_IA.Jump_IA"))
  (:`Started`
    (if (not (`self.IsDead`)) :!label _label
      (`self.Jump`)
      (`GameplayStatics.PlaySound2D` "/Game/sound/jump.jump" 1.0 1.0 0.0 null null)))
  (:`Completed`
    (`self.StopJumping` :!label _label_2)))

(event `jumpe`
  (goto _label))

(event `stopjkump`
  (goto _label_2))

(event `self.CapsuleComponent.OnComponentBeginOverlap`
  (params (OverlappedComponent :type "PrimitiveComponent Object Reference") (OtherActor :type "Actor Object Reference") (OtherComp :type "PrimitiveComponent Object Reference") (OtherBodyIndex :type Integer) (bFromSweep :type Boolean) (SweepResult :type "HitResult Structure (by ref)"))
  (if (`ActorComponent.ComponentHasTag` OtherComp "Damagebox")
    (`/Engine/EditorBlueprintResources/StandardMacros.DoOnce` false :!label _label_3
      (:`Completed`
        (set `self.IsDead` true)
        (`SceneComponent.K2_AddLocalOffset` (`self.Sprite`) (0.0 0.0 -10.0) false false)
        (`SceneComponent.K2_DetachFromComponent` (`self.Camera`) "KeepWorld" "KeepWorld" "KeepWorld" true)
        (`KismetSystemLibrary.Delay` 1.5)
        (bind _returnvalue (`|CreateWidget` "/Game/UI/GameOver.GameOver_C"))
        (`UserWidget.AddToViewport` _returnvalue 0)))))

(event `Fallen`
  (goto _label_3))

(event `Pause`
  (bind _returnvalue (`GameplayStatics.GetPlayerController` 0))
  (bind _returnvalue_2 (`GameplayStatics.GetPlayerController` 0))
  (if (not (`self.isPaused`))
    (bind _returnvalue_3 (`|CreateWidget` "/Game/UI/PauseMenu.PauseMenu_C" _returnvalue))
    (bind _output_get (set `self.PauseRef` _returnvalue_3))
    (`UserWidget.AddToViewport` _output_get 0)
    (`WidgetBlueprintLibrary.SetInputMode_GameAndUIEx` _returnvalue (`self.PauseRef`))
    (set `PlayerController.bShowMouseCursor` true (`GameplayStatics.GetPlayerController` 0))
    (`GameplayStatics.SetGamePaused` true)
    (else
      (set `self.isPaused` false)
      (`Widget.RemoveFromParent` (`self.PauseRef`))
      (`GameplayStatics.SetGamePaused` false)
      (`WidgetBlueprintLibrary.SetInputMode_GameOnly` _returnvalue_2)
      (set `PlayerController.bShowMouseCursor` false _returnvalue_2))))

(event `EnhancedInput|/Game/Input/Pause_IA`
  (params (ActionValue :type Boolean) (ElapsedSeconds :type "Float (double-precision)") (TriggeredSeconds :type "Float (double-precision)") (InputAction :type "InputAction Object Reference" :default "/Game/Input/Pause_IA.Pause_IA"))
  (:`Started`
    (`self.Pause`)))

(event `Key|P`
  (params (Key :type "Key Structure"))
  (:`Pressed`
    (`self.Pause`)))

(fn `UserConstructionScript`)